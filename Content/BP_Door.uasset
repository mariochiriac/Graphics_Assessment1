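; BP_Door is an interactable hinged door that stays locked, with a no-power prompt, until Unlock is called and turns its indicator light green.
; Its box trigger registers the door as the first-person character's CurrentInteractable and shows a state-dependent prompt, clearing both on exit.
; Interact opens an unlocked door once, hiding the prompt and rotating the Hinge through a timeline-driven lerp, with no closing logic.
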(event `Unlock`
  ; Event that unlocks door and changes door light
  (set `self.bUnlocked` true)
  (`LightComponent.SetLightColor` (`self.IndicatorLight`) (struct :`R` 0.127318 :`G` 1.0 :`B` 0.096677 :`A` 1.0) true))

(event `self.Box.OnComponentBeginOverlap`
  (params (OverlappedComponent :type "PrimitiveComponent Object Reference") (OtherActor :type "Actor Object Reference") (OtherComp :type "PrimitiveComponent Object Reference") (OtherBodyIndex :type Integer) (bFromSweep :type Boolean) (SweepResult :type "HitResult Structure (by ref)"))
  ; Player overlaps box collider, door is set as interactable object in character blueprint, prompt shown depending on condition
  (bind _asbp_first_person_character (cast `/Game/FirstPerson/Blueprints/BP_FirstPersonCharacter` OtherActor))
  (set `/Game/FirstPerson/Blueprints/BP_FirstPersonCharacter.CurrentInteractable` self _asbp_first_person_character)
  (if (`self.bUnlocked`)
    (if (`self.bOpen`)
      (`/Game/FirstPerson/Blueprints/BP_FirstPersonCharacter.HidePrompt` _asbp_first_person_character)
      (else
        (`/Game/FirstPerson/Blueprints/BP_FirstPersonCharacter.ShowPrompt` _asbp_first_person_character "Press E to open the door")))
    (else
      (`/Game/FirstPerson/Blueprints/BP_FirstPersonCharacter.ShowPrompt` _asbp_first_person_character "Locked - No power"))))

(event `self.Box.OnComponentEndOverlap`
  (params (OverlappedComponent :type "PrimitiveComponent Object Reference") (OtherActor :type "Actor Object Reference") (OtherComp :type "PrimitiveComponent Object Reference") (OtherBodyIndex :type Integer))
  ; Player not overlapping box collider anymore, hide prompt
  (bind _asbp_first_person_character (cast `/Game/FirstPerson/Blueprints/BP_FirstPersonCharacter` OtherActor))
  (set `/Game/FirstPerson/Blueprints/BP_FirstPersonCharacter.CurrentInteractable` null _asbp_first_person_character)
  (`/Game/FirstPerson/Blueprints/BP_FirstPersonCharacter.HidePrompt` _asbp_first_person_character))

(event `/Game/BPI_Interact.Interact`
  (if (`self.bUnlocked`)
    (if (not (`self.bOpen`))
      (set `self.bOpen` true)
      (bind _asbp_first_person_character (cast `/Game/FirstPerson/Blueprints/BP_FirstPersonCharacter` (`GameplayStatics.GetPlayerCharacter` 0)))
      (`/Game/FirstPerson/Blueprints/BP_FirstPersonCharacter.HidePrompt` _asbp_first_person_character)
      (bind (_direction _newtrack_0) (`Timeline|OpenDoor`)
        (:`Update`
          (`SceneComponent.K2_SetRelativeRotation` (`self.Hinge`) (`KismetMathLibrary.RLerp` (struct) (struct :`Yaw` -90.0) _newtrack_0) false false))))))

(fn `UserConstructionScript`)