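; BP_EndTrigger is a level-end trigger volume that finishes the level when the first-person player character enters its box.
; On the first valid overlap only, it hides the character's prompt, disables input on itself and fades screen and audio to a held end color.
; After the fade it shows the mouse cursor, adds the WBP_LevelComplete widget and switches to UI-only input.
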(event `self.Box.OnComponentBeginOverlap`
  (params (OverlappedComponent :type "PrimitiveComponent Object Reference") (OtherActor :type "Actor Object Reference") (OtherComp :type "PrimitiveComponent Object Reference") (OtherBodyIndex :type Integer) (bFromSweep :type Boolean) (SweepResult :type "HitResult Structure (by ref)"))
  (bind _returnvalue (`GameplayStatics.GetPlayerController` 0))
  (bind _asbp_first_person_character (cast `/Game/FirstPerson/Blueprints/BP_FirstPersonCharacter` OtherActor))
  (`/Engine/EditorBlueprintResources/StandardMacros.DoOnce` false
    (:`Completed`
      (`/Game/FirstPerson/Blueprints/BP_FirstPersonCharacter.HidePrompt` _asbp_first_person_character)
      (`self.DisableInput` _returnvalue)
      (`PlayerCameraManager.StartCameraFade` :`self` (`GameplayStatics.GetPlayerCameraManager` 0) :`ToAlpha` 1.0 :`Duration` 1.5 :`bShouldFadeAudio` true :`bHoldWhenFinished` true)
      (`KismetSystemLibrary.Delay` 1.5)
      (set `PlayerController.bShowMouseCursor` true _returnvalue)
      (bind _returnvalue_2 (`|CreateWidget` "/Game/WBP_LevelComplete.WBP_LevelComplete_C" _returnvalue))
      (`UserWidget.AddToViewport` _returnvalue_2 0)
      (`WidgetBlueprintLibrary.SetInputMode_UIOnlyEx` _returnvalue null))))

(fn `UserConstructionScript`)