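; Electrical panel puzzle that restores power to lights and unlocks a door when the player interacts with the breakers set correctly.
; A box overlap registers the panel as the first-person character's current interactable and shows a restore-power prompt while unpowered.
; Interact checks every switch against its intended state; success lights the linked lights and unlocks the door.
; Failure flickers the lights, resets all switches and shows a tripped-breaker prompt.
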(event `self.Box.OnComponentBeginOverlap`
  (params (OverlappedComponent :type "PrimitiveComponent Object Reference") (OtherActor :type "Actor Object Reference") (OtherComp :type "PrimitiveComponent Object Reference") (OtherBodyIndex :type Integer) (bFromSweep :type Boolean) (SweepResult :type "HitResult Structure (by ref)"))
  ; Manage user overlap electric panel, handle prompt and interaction start
  (bind _asbp_first_person_character (cast `/Game/FirstPerson/Blueprints/BP_FirstPersonCharacter` OtherActor))
  (set `/Game/FirstPerson/Blueprints/BP_FirstPersonCharacter.CurrentInteractable` self _asbp_first_person_character)
  (if (not (`self.bPowered`))
    (`/Game/FirstPerson/Blueprints/BP_FirstPersonCharacter.ShowPrompt` _asbp_first_person_character "Press E to restore power")))

(event `self.Box.OnComponentEndOverlap`
  (params (OverlappedComponent :type "PrimitiveComponent Object Reference") (OtherActor :type "Actor Object Reference") (OtherComp :type "PrimitiveComponent Object Reference") (OtherBodyIndex :type Integer))
  ; Manage user overlap electric panel, handle prompt and interaction start
  (bind _asbp_first_person_character (cast `/Game/FirstPerson/Blueprints/BP_FirstPersonCharacter` OtherActor))
  (set `/Game/FirstPerson/Blueprints/BP_FirstPersonCharacter.CurrentInteractable` null _asbp_first_person_character)
  (`/Game/FirstPerson/Blueprints/BP_FirstPersonCharacter.HidePrompt` _asbp_first_person_character))

(event `/Game/BPI_Interact.Interact`
  ; Manages interaction with panel, which hides the prompt, turns lights on and unlocks door
  (if (not (`self.bPowered`))
    (bind _asbp_first_person_character (cast `/Game/FirstPerson/Blueprints/BP_FirstPersonCharacter` (`GameplayStatics.GetPlayerCharacter` 0)))
    ; Circuit check: every breaker must match its bShouldBeOn. Any mismatch sets bCircuitOK false
    (set `self.bCircuitOK` true)
    (for _array_element (`self.Switches`)
      (if (!= (`/Game/BP_BreakerSwitch.bOn` _array_element) (`/Game/BP_BreakerSwitch.bShouldBeOn` _array_element))
        (set `self.bCircuitOK` false)))
    (if (`self.bCircuitOK`)
      (set `self.bPowered` true)
      (`/Game/FirstPerson/Blueprints/BP_FirstPersonCharacter.HidePrompt` _asbp_first_person_character)
      (for _array_element_2 (`self.Lights`)
        (`SceneComponent.SetVisibility` (`Light.LightComponent` _array_element_2) true false))
      (`/Game/BP_Door.Unlock` (`self.BP_Door`))
      (else
        ; Wrong combination: lights flicker on then off, every breaker resets, prompt tells the player it tripped
        (for _array_element_3 (`self.Lights`)
          (`SceneComponent.SetVisibility` (`Light.LightComponent` _array_element_3) true false))
        (`KismetSystemLibrary.Delay` 0.35)
        (for _array_element_4 (`self.Lights`)
          (`SceneComponent.SetVisibility` (`Light.LightComponent` _array_element_4) false false))
        (for _array_element_5 (`self.Switches`)
          (`/Game/BP_BreakerSwitch.ResetSwitch` _array_element_5))
        (`/Game/FirstPerson/Blueprints/BP_FirstPersonCharacter.ShowPrompt` _asbp_first_person_character (`KismetTextLibrary.Conv_StringToText` "Breaker tripped. Check the circuit breakers."))))))

(fn `UserConstructionScript`)